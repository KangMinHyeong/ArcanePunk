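; BP_SwapDashTrail is a short-lived afterimage actor for the swap dash effect, showing a frozen copy of a character's pose.
; Init copies the pose from the given skeletal component onto a PoseableMesh, optionally replacing every material with a uniform color one, and sets Intensity.
; A timeline then animates Opacity, plus Color in uniform mode, and destroys the actor when finished.
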(event Custom|Init
  (params (NewParam :type Skeletal%20Mesh%20Component%20Object%20Reference))
  (bind _poseablemesh (Variables|Default|GetPoseableMesh))
  (if (Variables|Default|GetUniform)
    ;[1 1 1] Uniform Material Setting
    (for (_ _array_index) (Rendering|Material|GetMaterials (Variables|Default|GetPoseableMesh))
      (Rendering|Material|SetMaterial (Variables|Default|GetPoseableMesh) _array_index "/Game/Asset/Effect/BP/BP_Dash/M_SwapDashTrail_Uniform_Color.M_SwapDashTrail_Uniform_Color")))
  (Class|PoseableMeshComponent|CopyPosefromSkeletalComponent _poseablemesh NewParam)
  (Rendering|Material|SetScalarParameterValueonMaterials _poseablemesh "Intensity" (Variables|Default|GetIntensity))
  (bind (_direction _opacity _color) (Timeline|Timeline PlayFromStart)
    (:Update
      (Rendering|Material|SetScalarParameterValueonMaterials _poseablemesh "Opacity" _opacity)
      (if (Variables|Default|GetUniform)
        (Rendering|Material|SetVectorParameterValueonMaterials _poseablemesh "Color" (Math|Conversions|ToVector(LinearColor) _color))))
    (:Finished
      (Actor|DestroyActor))))

(event EventBeginPlay)

(event Collision|EventActorBeginOverlap
  (params (OtherActor :type Actor%20Object%20Reference)))

(event EventTick
  (params (DeltaSeconds :type Float%20%28single-precision%29)))

(fn ConstructionScript)