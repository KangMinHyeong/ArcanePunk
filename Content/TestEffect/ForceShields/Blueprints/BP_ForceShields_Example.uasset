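; BP_ForceShields_Example is a demo force shield that shows impact effects on a sphere.
; The construction script applies the shield material and scale.
; BeginPlay loops every two seconds, adding three static meshes at billboard positions, each bound to destroy on hit.
; The Hit event, limited to once per frame, spawns a child actor and sends it the relative hit location, ring modifiers and material-derived fade and color.
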(event Custom|Destroy#3
  (params (HitComponent :type Primitive%20Component%20Object%20Reference) (OtherActor :type Actor%20Object%20Reference) (OtherComp :type Primitive%20Component%20Object%20Reference) (NormalImpulse :type Vector) (Hit :type Hit%20Result%20Structure%20%28by%20ref%29))
  (Components|DestroyComponent (stale EventBeginPlay _returnvalue_3)))

(event Custom|Destroy#1
  (params (HitComponent :type Primitive%20Component%20Object%20Reference) (OtherActor :type Actor%20Object%20Reference) (OtherComp :type Primitive%20Component%20Object%20Reference) (NormalImpulse :type Vector) (Hit :type Hit%20Result%20Structure%20%28by%20ref%29))
  (Components|DestroyComponent (stale EventBeginPlay _returnvalue)))

(event Custom|Destroy#2
  (params (HitComponent :type Primitive%20Component%20Object%20Reference) (OtherActor :type Actor%20Object%20Reference) (OtherComp :type Primitive%20Component%20Object%20Reference) (NormalImpulse :type Vector) (Hit :type Hit%20Result%20Structure%20%28by%20ref%29))
  (Components|DestroyComponent (stale EventBeginPlay _returnvalue_2)))

(event EventBeginPlay
  (bind _returnvalue (AddComponent|AddStaticMeshComponent false (Transformation|GetRelativeTransform (Variables|Default|GetBillboard)) :!label _label))
  (Collision|BindEventtoOnComponentHit _returnvalue (delegate Custom|Destroy#1))
  (bind _returnvalue_2 (AddComponent|AddStaticMeshComponent false (Transformation|GetRelativeTransform (Variables|Default|GetBillboard1))))
  (Collision|BindEventtoOnComponentHit _returnvalue_2 (delegate Custom|Destroy#2))
  (bind _returnvalue_3 (AddComponent|AddStaticMeshComponent false (Transformation|GetRelativeTransform (Variables|Default|GetBillboard2))))
  (Collision|BindEventtoOnComponentHit _returnvalue_3 (delegate Custom|Destroy#3))
  (Utilities|FlowControl|Delay 2.0)
  (goto _label))

(event Collision|EventHit
  (params (MyComp :type Primitive%20Component%20Object%20Reference) (Other :type Actor%20Object%20Reference) (OtherComp :type Primitive%20Component%20Object%20Reference) (bSelfMoved :type Boolean) (HitLocation :type Vector :default "0, 0, 0") (HitNormal :type Vector :default "0, 0, 0") (NormalImpulse :type Vector :default "0, 0, 0") (Hit :type Hit%20Result%20Structure%20%28by%20ref%29))
  (if (not (Variables|Default|GetBlockSpawn))
    (Variables|Default|SetBlockSpawn true)
    (bind _returnvalue (AddComponent|AddChildActorComponent false (Math|Transform|MakeTransform "0, 0, 0" "0, 0, 0" (Variables|/Script/Engine.SceneComponent|GetRelativeScale3D (Variables|Default|GetSphere)))))
    (bind _returnvalue_2 (Rendering|Material|CreateDynamicMaterialInstance (Variables|Default|GetSphere) 0 (Variables|Default|GetMaterial) "None" :!class /Script/Engine.PrimitiveComponent))
    (bind _returnvalue_3 (Rendering|Material|GetScalarParameterValue _returnvalue_2 "Fade Opacity" :!class /Script/Engine.MaterialInstanceDynamic))
    (bind _returnvalue_4 (Rendering|Material|GetScalarParameterValue _returnvalue_2 "Fade Distance" :!class /Script/Engine.MaterialInstanceDynamic))
    (bind _returnvalue_5 (Rendering|Material|GetVectorParameterValue _returnvalue_2 "Color_01" :!class /Script/Engine.MaterialInstanceDynamic))
    (Class|HitInterface|ShieldHit(Message) (Variables|/Script/Engine.ChildActorComponent|GetChildActor _returnvalue) (- HitLocation (Transformation|GetWorldLocation (Variables|Default|GetSphere))) (Variables|Default|GetShield%20Scale) (Variables|Default|GetHit%20Ring%20Size) (Variables|Default|GetHit%20Ring%20Width) _returnvalue_4 _returnvalue_3 (Math|Conversions|ToColor(LinearColor) _returnvalue_5) false)
    (Utilities|FlowControl|Delay 0.0)
    (Variables|Default|SetBlockSpawn false)))

(fn ConstructionScript
  (Rendering|Material|SetMaterial (Variables|Default|GetSphere) 0 (Variables|Default|GetMaterial))
  (Transformation|SetActorRelativeScale3D (Math|Conversions|ToVector(Float) (Variables|Default|GetShield%20Scale))))