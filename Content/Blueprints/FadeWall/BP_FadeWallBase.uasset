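; BP_FadeWallBase is a base wall actor that fades its SkinMesh out and back in on demand.
; The construction script caches the original materials and builds dynamic instances from the Fade material array.
; FadeOut swaps in those instances and plays a timeline driving their "Fade" scalar, while Fadein reverses it.
; Finishing at 1 restores the original materials; both endpoints set the mesh's Visibility collision response to Ignore.
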(event EventBeginPlay)

(event Collision|EventActorBeginOverlap
  (params (OtherActor :type Actor%20Object%20Reference)))

(event EventTick
  (params (DeltaSeconds :type Float%20%28single-precision%29)))

(event EventFadein
  (bind _skinmesh (Variables|Default|GetSkinMesh))
  (bind _새_트랙_0 (Timeline|타임라인 Reverse)
    (:Update
      (for _array_element (Variables|Default|GetDynamic)
        (Rendering|Material|SetScalarParameterValue _array_element "Fade" _새_트랙_0 :!class /Script/Engine.MaterialInstanceDynamic)))
    (:Finished
      (if (>= _새_트랙_0 1.0)
        (for (_array_element_2 _array_index) (Variables|Default|GetOrigin)
          (Rendering|Material|SetMaterial (Variables|Default|GetSkinMesh) _array_index _array_element_2)
          (Collision|SetCollisionResponsetoChannel _skinmesh "ECC_Visibility" "ECR_Ignore"))
        (elif (<= _새_트랙_0 0.0)
          (Collision|SetCollisionResponsetoChannel _skinmesh "ECC_Visibility" "ECR_Ignore"))))))

(event EventFadeOut
  (bind _skinmesh (Variables|Default|GetSkinMesh))
  (for (_array_element _array_index) (Variables|Default|GetDynamic)
    (Rendering|Material|SetMaterial (Variables|Default|GetSkinMesh) _array_index _array_element)
    (bind _새_트랙_0 (Timeline|타임라인 Play)
      (:Update
        (for _array_element_2 (Variables|Default|GetDynamic)
          (Rendering|Material|SetScalarParameterValue _array_element_2 "Fade" _새_트랙_0 :!class /Script/Engine.MaterialInstanceDynamic)))
      (:Finished
        (if (>= _새_트랙_0 1.0)
          (for (_array_element_3 _array_index_2) (Variables|Default|GetOrigin)
            (Rendering|Material|SetMaterial (Variables|Default|GetSkinMesh) _array_index_2 _array_element_3)
            (Collision|SetCollisionResponsetoChannel _skinmesh "ECC_Visibility" "ECR_Ignore"))
          (elif (<= _새_트랙_0 0.0)
            (Collision|SetCollisionResponsetoChannel _skinmesh "ECC_Visibility" "ECR_Ignore")))))))

(fn ConstructionScript
  (Utilities|Array|Clear (Variables|Default|GetDynamic))
  (Variables|Default|SetOrigin (Rendering|Material|GetMaterials (Variables|Default|GetSkinMesh)))
  (for _array_element (Variables|Default|GetFade)
    (bind _returnvalue (Rendering|Material|CreateDynamicMaterialInstance _array_element "None" "None" :!class /Script/Engine.KismetMaterialLibrary))
    (Utilities|Array|AddUnique (Variables|Default|GetDynamic) _returnvalue)))