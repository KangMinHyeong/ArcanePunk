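; BP_SwordImpact_2 is a skill actor that carries a Niagara effect, BaseEffect, and receives particle data back from it.
; On BeginPlay it passes itself to the effect as the collision callback object, under both User_Collision and Collision parameter names.
; The ParticleData event loops over the exported particles and only prints each position on screen as debug output, with no hit logic.
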(event EventBeginPlay
  (bind _self self)
  (bind _baseeffect (Variables|Default|GetBaseEffect))
  (Niagara|SetNiagaraVariable(Object) _baseeffect "User_Collision" self)
  (Niagara|SetNiagaraVariable(Object) _baseeffect "Collision" _self)
  (Class|NiagaraComponent|SetVariableObject _baseeffect "Collision" _self))

(event Collision|EventActorBeginOverlap
  (params (OtherActor :type Actor%20Object%20Reference)))

(event EventTick
  (params (DeltaSeconds :type Float%20%28single-precision%29)))

(event EventParticleData
  (params (Data :type Array%20of%20Basic%20Particle%20Data%20Structures) (NiagaraSystem :type Niagara%20System%20Object%20Reference) (SimulationPositionOffset :type Vector%20%28by%20ref%29 :default "0, 0, 0"))
  (for _array_element Data
    (Development|PrintString (Utilities|String|ToString(Vector) (.Position (Utilities|Struct|BreakBasicParticleData _array_element))) true true "(R=0.000000,G=0.660000,B=1.000000,A=1.000000)" 5e+01)))

(fn ConstructionScript)