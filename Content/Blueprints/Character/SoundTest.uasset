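; SoundTest is an actor that appears to be a test bed for attached sounds and Niagara particle data callbacks.
; It spawns the default step sound on its Cube every Tick, and an uncalled MyFunction repeats that spawn.
; Overlap by an ArcanePunkCharacter spawns an ArcaneRain Niagara system at the actor.
; BeginPlay registers the actor as a Niagara CustomObject, and its ParticleData event prints received particle positions.
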(event EventBeginPlay
  (Niagara|SetNiagaraVariable(Object) "CustomObject" self))

(event EventParticleData
  (params (Data :type Array%20of%20Basic%20Particle%20Data%20Structures) (NiagaraSystem :type Niagara%20System%20Object%20Reference) (SimulationPositionOffset :type Vector%20%28by%20ref%29 :default "0, 0, 0"))
  (for _array_element Data
    (Development|PrintString (Utilities|String|ToString(Vector) (.Position (Utilities|Struct|BreakBasicParticleData _array_element))))))

(event EventTick
  (params (DeltaSeconds :type Float%20%28single-precision%29))
  (Audio|SpawnSoundAttached "/Game/Asset/Sound/Step/Default/Sound_Step_Default.Sound_Step_Default" (Variables|Default|GetCube) "None" "0, 0, 0" "0, 0, 0" "KeepRelativeOffset" false 1.0 1.0 0.0 0 0))

(event Collision|EventActorBeginOverlap
  (params (OtherActor :type Actor%20Object%20Reference))
  (Utilities|Casting|CastToArcanePunkCharacter OtherActor)
  (Niagara|SpawnSystematLocation "/Game/Asset/Effect/ArcaneRain_Origin_Fixed.ArcaneRain_Origin_Fixed" (Transformation|GetActorLocation)))

(fn ConstructionScript)

(fn MyFunction
  (Audio|SpawnSoundAttached "/Game/Asset/Sound/Step/Default/Sound_Step_Default.Sound_Step_Default" (Variables|Default|GetCube) "None" "0, 0, 0" "0, 0, 0" "KeepRelativeOffset" false 1.0 1.0 0.0 0 0))